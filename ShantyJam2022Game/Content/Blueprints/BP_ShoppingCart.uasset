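; BP_ShoppingCart is a player-controlled shopping cart actor that moves sideways along the Y axis.
; Left/A and Right/D key presses, gated by IsMovementEnabled, teleport it a fixed step without sweeping.
; Each press also flips the cart 180 degrees when its root rotation does not match the travel direction.
; An unconnected chain would spawn BP_MrFrog beside the Plane and store it in MrFrogImage, but never runs.
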(event EventBeginPlay)

(event Input|KeyboardEvents|A
  (params (Key :type Key%20Structure :default "None"))
  (bind _self self)
  (:Pressed
    (if (Variables|Default|GetbIsMovementEnabled?)
      (Transformation|AddActorWorldOffset "0,-20.000000, 0" false true)
      (if (not (Utilities|Operators|EqualEqual (Transformation|GetWorldRotation (Variables|Default|GetDefaultSceneRoot _self)) "0,180.000000,0" 0.2))
        (Class|Actor|AddActorWorldRotation _self "0,180.000000, 0")))))

(event Input|KeyboardEvents|D
  (params (Key :type Key%20Structure :default "None"))
  (bind _self self)
  (:Pressed
    (if (Variables|Default|GetbIsMovementEnabled?)
      (Transformation|AddActorWorldOffset "0,20.000000, 0" false true)
      (if (not (Utilities|Operators|EqualEqual :A (Transformation|GetWorldRotation (Variables|Default|GetDefaultSceneRoot _self)) :ErrorTolerance 0.2))
        (Class|Actor|AddActorWorldRotation _self "0,-180.000000, 0")))))

(event Input|KeyboardEvents|Left
  (params (Key :type Key%20Structure :default "None"))
  (bind _self self)
  (:Pressed
    (if (Variables|Default|GetbIsMovementEnabled?)
      (Transformation|AddActorWorldOffset "0,-20.000000, 0" false true)
      (if (not (Utilities|Operators|EqualEqual (Transformation|GetWorldRotation (Variables|Default|GetDefaultSceneRoot _self)) "0,180.000000,0" 0.2))
        (Class|Actor|AddActorWorldRotation _self "0,180.000000, 0")))))

(event Input|KeyboardEvents|Right
  (params (Key :type Key%20Structure :default "None"))
  (bind _self self)
  (:Pressed
    (if (Variables|Default|GetbIsMovementEnabled?)
      (Transformation|AddActorWorldOffset "0,20.000000, 0" false true)
      (if (not (Utilities|Operators|EqualEqual :A (Transformation|GetWorldRotation (Variables|Default|GetDefaultSceneRoot _self)) :ErrorTolerance 0.2))
        (Class|Actor|AddActorWorldRotation _self "0,-180.000000, 0")))))

(fn ConstructionScript)