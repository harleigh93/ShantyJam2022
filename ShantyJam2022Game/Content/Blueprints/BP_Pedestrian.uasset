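; BP_Pedestrian is a pedestrian actor with a Frog component that walks along negative world X until the Frogger character hits it.
; While alive, Tick applies a fixed per-frame offset and a ping-ponging timeline rocks the component's pitch.
; The first player overlap marks it dead, enables physics and calls OnPedestrianHurt.
; Once dead, Tick pushes the body along +Y with acceleration-based force, under a velocity cap.
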(event EventTick
  (params (DeltaSeconds :type Float%20%28single-precision%29))
  (if (not (Variables|Default|GetisDead))
    (Transformation|AddActorWorldOffset "-0.500000,0.000000, 0")
    (bind _newtrack_0 (Timeline|Timeline_0 Play)
      (:Update
        (if (not (Variables|Default|GetisDead))
          (Transformation|SetRelativeRotation (Variables|Default|GetFrog) (Math|Rotator|MakeRotator 0.0 _newtrack_0 0.0) false false)))
      (:Finished
        (if (Variables|Default|GetDirection)
          (Variables|Default|SetDirection false)
          (Timeline|Timeline_0 PlayFromStart)
          (else
            (Variables|Default|SetDirection true)
            (Timeline|Timeline_0 ReverseFromEnd)))))
    (elif (< (Math|Vector|VectorLength (Transformation|GetComponentVelocity (Variables|Default|GetFrog))) 5e+04)
      (Physics|AddForce (Variables|Default|GetFrog) "0,20.000000, 0" "None" true))))

(event Collision|EventActorBeginOverlap
  (params (OtherActor :type Actor%20Object%20Reference))
  (Utilities|Casting|CastToBP_FroggerCharacter OtherActor)
  (Utilities|FlowControl|DoOnce false
    (:Completed
      (Variables|Default|SetisDead true)
      (Physics|SetSimulatePhysics (Variables|Default|GetFrog) true)
      (Default|CallOnPedestrianHurt))))

(fn ConstructionScript)