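; BP_MovingLog is a Frogger-style log that slides along negative X and carries the player riding it.
; Tick, throttled by a Delay of twice DeltaSeconds, applies a fixed, frame-rate-dependent offset without sweep.
; Box overlaps set or clear the BP_FroggerCharacter reference, which receives the same offset.
; Past NegativeBound, the log wraps to PositiveBound at its saved starting Y and Z.
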(event OnComponentBeginOverlap(Box)
  (params (OverlappedComponent :type Primitive%20Component%20Object%20Reference) (OtherActor :type Actor%20Object%20Reference) (OtherComp :type Primitive%20Component%20Object%20Reference) (OtherBodyIndex :type Integer) (bFromSweep :type Boolean) (SweepResult :type Hit%20Result%20Structure%20%28by%20ref%29))
  (bind _asbp_frogger_character (Utilities|Casting|CastToBP_FroggerCharacter OtherActor))
  (Variables|Default|SetPlayer _asbp_frogger_character))

(event OnComponentEndOverlap(Box)
  (params (OverlappedComponent :type Primitive%20Component%20Object%20Reference) (OtherActor :type Actor%20Object%20Reference) (OtherComp :type Primitive%20Component%20Object%20Reference) (OtherBodyIndex :type Integer))
  (Utilities|Casting|CastToBP_FroggerCharacter OtherActor)
  (Variables|Default|SetPlayer 0))

(event EventBeginPlay
  (bind _returnvalue (Transformation|GetActorLocation))
  (Variables|Default|SetSavedY (.y _returnvalue))
  (Variables|Default|SetSavedZ (.z _returnvalue)))

(event Collision|EventActorBeginOverlap
  (params (OtherActor :type Actor%20Object%20Reference)))

(event EventTick
  (params (DeltaSeconds :type Float%20%28single-precision%29))
  (Utilities|FlowControl|Delay (* DeltaSeconds 2.0))
  (Transformation|AddActorWorldOffset "-3.000000,0.000000, 0")
  (Utilities|IsValid (Variables|Default|GetPlayer)
    (:Is%20Valid
      (Transformation|AddActorWorldOffset (Variables|Default|GetPlayer) "-3.000000,0.000000, 0"))
    (:Is%20Not%20Valid
      _))
  (if (< (.x (Transformation|GetActorLocation)) (Variables|Default|GetNegativeBound))
    (Transformation|SetActorLocation (Math|Vector|MakeVector (Variables|Default|GetPositiveBound) (Variables|Default|GetSavedY) (Variables|Default|GetSavedZ)) false false)))

(fn ConstructionScript)