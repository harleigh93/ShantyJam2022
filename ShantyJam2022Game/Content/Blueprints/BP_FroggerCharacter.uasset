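; Player character for a Frogger-style game that hops forward and back in fixed steps.
; On BeginPlay in ThirdPersonMap, it blends the player's view to the first CameraActor found in the level.
; W and S presses, gated by IsMovementEnabled, offset the actor along world Y by teleporting without sweep, bypassing collision and regular character movement.
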(event EventBeginPlay
  (bind _returnvalue (Game|GetCurrentLevelName true))
  (if (Utilities|Enum|Equal(Enum) _returnvalue "ThirdPersonMap")
    (bind _outactors (Actor|GetAllActorsOfClass "/Script/Engine.CameraActor"))
    (Game|Player|SetViewTargetwithBlend (Game|GetPlayerController 0) (Utilities|Array|Get(acopy) _outactors) 1.0 "VTBlend_Linear" 0.0 false)))

(event Input|KeyboardEvents|W
  (params (Key :type Key%20Structure :default "None"))
  (:Pressed
    (if (Variables|Default|GetisMovementEnabled?)
      (Transformation|AddActorWorldOffset "0,50.000000, 0" false true))))

(event Input|KeyboardEvents|S
  (params (Key :type Key%20Structure :default "None"))
  (:Pressed
    (if (Variables|Default|GetisMovementEnabled?)
      (Transformation|AddActorWorldOffset "0,-50.000000, 0" false true))))

(fn ConstructionScript)