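; BP_CroakscoSpawnItem is a falling food pickup that the player catches with a shopping cart.
; On BeginPlay it passes its food type to a FoodPickup widget component to set the image, then starts a looping timer that steps it downward by teleporting at fixed intervals.
; When its box overlaps a BP_ShoppingCart, it fires a food-caught dispatcher with that type and destroys itself.
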(event OnComponentBeginOverlap(Box)
  (params (OverlappedComponent :type Primitive%20Component%20Object%20Reference) (OtherActor :type Actor%20Object%20Reference) (OtherComp :type Primitive%20Component%20Object%20Reference) (OtherBodyIndex :type Integer) (bFromSweep :type Boolean) (SweepResult :type Hit%20Result%20Structure%20%28by%20ref%29))
  (Utilities|Casting|CastToBP_ShoppingCart OtherActor)
  (Default|CallFoodItemCaught (Variables|Default|GetFoodToSpawn))
  (Actor|DestroyActor self))

(event Custom|Food%20Falling
  (Transformation|AddActorWorldOffset (Math|Vector|MakeVector 0.0 0.0 -15.0) false true))

(event EventBeginPlay
  (bind _asfood_pickup (Utilities|Casting|CastToFoodPickup (UserInterface|GetUserWidgetObject (Variables|Default|GetFoodItem))))
  (Variables|Default|SetFoodWidgetRef _asfood_pickup)
  (Variables|/Game/Widgets/FoodPickup.FoodPickup_C|SetFoodType (Variables|Default|GetFoodWidgetRef) (Variables|Default|GetFoodToSpawn))
  (Default|HandleFoodImage (Variables|Default|GetFoodWidgetRef))
  (Utilities|Time|SetTimerbyEvent (delegate Custom|Food%20Falling) 0.15 true))

(fn ConstructionScript)